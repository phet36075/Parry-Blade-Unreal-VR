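; MyBlade_BP is a blade actor that gives sound and glow feedback when it hits during a VR swing.
; BladeHitBox overlaps count only while the player's VRPawn reports IsSwinging, with no filter on the overlapped actor.
; Each one spawns a random swing-ring cue at the mesh, picked from the InfBladeSwingRing array through a switch.
; It also restarts GlowTimeline, which drives the GlowIntensity material parameter.
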(event `self.ReceiveBeginPlay`)

(event `self.BladeHitBox.OnComponentBeginOverlap`
  (params (OverlappedComponent :type "PrimitiveComponent Object Reference") (OtherActor :type "Actor Object Reference") (OtherComp :type "PrimitiveComponent Object Reference") (OtherBodyIndex :type Integer) (bFromSweep :type Boolean) (SweepResult :type "HitResult Structure (by ref)"))
  (bind _asvrpawn (cast `/Game/VRTemplate/Blueprints/VRPawn` (`GameplayStatics.GetPlayerPawn` 0)))
  (if (`/Game/VRTemplate/Blueprints/VRPawn.IsSwinging` _asvrpawn)
    (`self.Play InfBladeSwingRing`)
    (bind (_direction _glowintensity) (`Timeline|GlowTimeline` :!via `PlayFromStart`)
      (:`Update`
        (`MeshComponent.SetScalarParameterValueOnMaterials` (`self.StaticMesh`) "GlowIntensity" _glowintensity)))))

(event `Play InfBladeSwingRing`
  (bind _returnvalue (`SceneComponent.K2_GetComponentLocation` (`self.StaticMesh`)))
  (switch `/Game/Sounds/InfBlade_SwingRing/InfBladeSwingRing` (`KismetArrayLibrary.Array_Random` (`self.InfBladeSwingRing`))
    (:`NewEnumerator0`
      (`GameplayStatics.SpawnSoundAtLocation` "/Game/Sounds/InfBlade_SwingRing/InfBlade_SwingRingB05_1_Cue.InfBlade_SwingRingB05_1_Cue" _returnvalue (struct) 1.0 1.0 0.0 null null))
    (:`NewEnumerator1`
      (`GameplayStatics.SpawnSoundAtLocation` "/Game/Sounds/InfBlade_SwingRing/InfBlade_SwingRingC01_1_Cue.InfBlade_SwingRingC01_1_Cue" _returnvalue (struct) 1.0 1.0 0.0 null null))
    (:`NewEnumerator2`
      (`GameplayStatics.SpawnSoundAtLocation` "/Game/Sounds/InfBlade_SwingRing/InfBlade_SwingRingC02_1_Cue.InfBlade_SwingRingC02_1_Cue" _returnvalue (struct) 1.0 1.0 0.0 null null))
    (:`NewEnumerator3`
      (`GameplayStatics.SpawnSoundAtLocation` "/Game/Sounds/InfBlade_SwingRing/InfBlade_SwingRingC06_1_Cue.InfBlade_SwingRingC06_1_Cue" _returnvalue (struct) 1.0 1.0 0.0 null null))
    (:`NewEnumerator4`
      (`GameplayStatics.SpawnSoundAtLocation` "/Game/Sounds/InfBlade_SwingRing/InfBlade_SwingRingC05_1_Cue.InfBlade_SwingRingC05_1_Cue" _returnvalue (struct) 1.0 1.0 0.0 null null))
    (:`NewEnumerator5`
      (`GameplayStatics.SpawnSoundAtLocation` "/Game/Sounds/InfBlade_SwingRing/InfBlade_SwingRingC04_1_Cue.InfBlade_SwingRingC04_1_Cue" _returnvalue (struct) 1.0 1.0 0.0 null null))
    (:`NewEnumerator6`
      (`GameplayStatics.SpawnSoundAtLocation` "/Game/Sounds/InfBlade_SwingRing/InfBlade_SwingRingC03_1_Cue.InfBlade_SwingRingC03_1_Cue" _returnvalue (struct) 1.0 1.0 0.0 null null))))

(fn `UserConstructionScript`)